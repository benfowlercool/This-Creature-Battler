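; Gameplay ability for Sproot's dig: toggles the character between normal and buried states, tracked by the Burried gameplay tag.
; Burying swaps the mesh to a skull, applies the creature's burrow speed and disables jumping.
; Reactivating while buried restores creature defaults, as does ability end.
; Fast looping timers drive tag-based cooldown and burrow-duration helpers, ending the ability when their tags clear, with a gate flag guarding the burrow timer's end.
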(event `EndCooldown`
  (bind _as_tpc (`self.As TPC`))
  (`self.CooldownTimerAbility1` (struct :`TagName` "Attacking?.Ability2") (`/Game/Dynamic/ThirdPerson/Blueprints/BP_ThirdPersonCharacter.Ability2MC` _as_tpc))
  (if (not (`BlueprintGameplayTagLibrary.HasTag` (`/Game/Dynamic/ThirdPerson/Blueprints/BP_ThirdPersonCharacter.GameplayTagManager` _as_tpc) (struct :`TagName` "Attacking?.Ability2")))
    (`self.K2_EndAbility`)))

(event `self.K2_ActivateAbility`
  (bind _as_tpc (`self.As TPC`))
  (bind _as_tpc_2 (`self.As TPC`))
  (bind _as_tpc_3 (`self.As TPC`))
  (bind _as_tpc_4 (`self.As TPC`))
  (bind _thiscreature (`/Game/Dynamic/ThirdPerson/Blueprints/BP_ThirdPersonCharacter.ThisCreature` _as_tpc_2))
  (bind _asbp_third_person_character (cast `/Game/Dynamic/ThirdPerson/Blueprints/BP_ThirdPersonCharacter` (`self.GetAvatarActorFromActorInfo`)))
  (bind _output_get (set `self.As TPC` _asbp_third_person_character))
  (`self.K2_CommitAbility`)
  (bind _gameplaytagmanager (`/Game/Dynamic/ThirdPerson/Blueprints/BP_ThirdPersonCharacter.GameplayTagManager` _output_get))
  (`BlueprintGameplayTagLibrary.AddGameplayTag` _gameplaytagmanager (struct :`TagName` "Attacking?.Ability2"))
  (if (`BlueprintGameplayTagLibrary.HasTag` _gameplaytagmanager (struct :`TagName` "Burried") true)
    (set `self.EndMethodGate` true)
    (set `self.A1Timer` (`/Game/Dynamic/ThirdPerson/Blueprints/BP_ThirdPersonCharacter.Ability2MC` (`self.As TPC`)))
    (set `CharacterMovementComponent.MaxWalkSpeed` (`/Game/Dynamic/Creatures/CreatureDataAsset.Speed` _thiscreature) (`Character.CharacterMovement` _as_tpc_2))
    (set `Character.JumpMaxCount` (`/Game/Dynamic/Creatures/CreatureDataAsset.NumOfJumps` _thiscreature) _as_tpc)
    (`SkeletalMeshComponent.SetSkeletalMeshAsset` (`Character.Mesh` _as_tpc) (`/Game/Dynamic/Creatures/CreatureDataAsset.Model` _thiscreature))
    (`BlueprintGameplayTagLibrary.RemoveGameplayTag` (`/Game/Dynamic/ThirdPerson/Blueprints/BP_ThirdPersonCharacter.GameplayTagManager` _as_tpc_2) (struct :`TagName` "Burried"))
    (`KismetSystemLibrary.K2_SetTimerDelegate` (delegate `EndCooldown`) 0.001 true)
    (else
      (set `self.A1Timer` (`/Game/Dynamic/ThirdPerson/Blueprints/BP_ThirdPersonCharacter.Ability2MC` _as_tpc_4))
      (`SkeletalMeshComponent.SetSkeletalMeshAsset` (`Character.Mesh` _as_tpc_4) "/Game/Static/Characters/Models/Skull/Skull.Skull")
      (set `CharacterMovementComponent.MaxWalkSpeed` (`/Game/Dynamic/Creatures/CreatureDataAsset.BurrySpeed` (`/Game/Dynamic/ThirdPerson/Blueprints/BP_ThirdPersonCharacter.ThisCreature` _as_tpc_3)) (`Character.CharacterMovement` _as_tpc_3))
      (set `Character.JumpMaxCount` 0 _as_tpc_3)
      (`KismetSystemLibrary.K2_SetTimerDelegate` (delegate `UpdateTimer`) 0.001 true)
      (set `self.BuryCC` (`/Game/Dynamic/ThirdPerson/Blueprints/BP_ThirdPersonCharacter.BurryMC` (`self.As TPC`)))
      (`KismetSystemLibrary.K2_SetTimerDelegate` (delegate `UnBurryTimer`) 0.001 true)
      (`BlueprintGameplayTagLibrary.AddGameplayTag` (`/Game/Dynamic/ThirdPerson/Blueprints/BP_ThirdPersonCharacter.GameplayTagManager` (`self.As TPC`)) (struct :`TagName` "Burried")))))

(event `UpdateTimer`
  (`self.CooldownTimerAbility1` (struct :`TagName` "Attacking?.Ability2") (`/Game/Dynamic/ThirdPerson/Blueprints/BP_ThirdPersonCharacter.Ability2MC` (`self.As TPC`))))

(event `UnBurryTimer`
  (`self.BurryTimer` (struct :`TagName` "Burried") (`/Game/Dynamic/ThirdPerson/Blueprints/BP_ThirdPersonCharacter.BurryMC` (`self.As TPC`)))
  (if (`BlueprintGameplayTagLibrary.HasTag` (`/Game/Dynamic/ThirdPerson/Blueprints/BP_ThirdPersonCharacter.GameplayTagManager` (`self.As TPC`)) (struct :`TagName` "Burried"))
    _
    (elif (not (`self.EndMethodGate`))
      (`self.K2_EndAbility`))))

(event `self.K2_OnEndAbility`
  (params (bWasCancelled :type Boolean))
  (bind _as_tpc (`self.As TPC`))
  (bind _as_tpc_2 (`self.As TPC`))
  (bind _thiscreature (`/Game/Dynamic/ThirdPerson/Blueprints/BP_ThirdPersonCharacter.ThisCreature` _as_tpc))
  (set `CharacterMovementComponent.MaxWalkSpeed` (`/Game/Dynamic/Creatures/CreatureDataAsset.Speed` _thiscreature) (`Character.CharacterMovement` _as_tpc))
  (set `Character.JumpMaxCount` (`/Game/Dynamic/Creatures/CreatureDataAsset.NumOfJumps` _thiscreature) _as_tpc_2)
  (`SkeletalMeshComponent.SetSkeletalMeshAsset` (`Character.Mesh` _as_tpc_2) (`/Game/Dynamic/Creatures/CreatureDataAsset.Model` _thiscreature))
  (`BlueprintGameplayTagLibrary.RemoveGameplayTag` (`/Game/Dynamic/ThirdPerson/Blueprints/BP_ThirdPersonCharacter.GameplayTagManager` _as_tpc) (struct :`TagName` "Burried")))