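; Gameplay ability that lets the Sproot pop out of the ground when the avatar third-person character is buried.
; It clears the buried flag and restores walk speed, jump count and skeletal mesh from the character's creature data.
; Movement then stops and drops to a crawl for a short fixed delay before full speed returns and the ability ends.
; If the character is not buried, it ends immediately.
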(event `self.K2_ActivateAbility`
  (bind _as_tpc (`self.As TPC`))
  (bind _as_tpc_2 (`self.As TPC`))
  (bind _as_tpc_3 (`self.As TPC`))
  (bind _charactermovement (`Character.CharacterMovement` _as_tpc_2))
  (bind _thiscreature (`/Game/Dynamic/ThirdPerson/Blueprints/BP_ThirdPersonCharacter.ThisCreature` _as_tpc_3))
  (bind _asbp_third_person_character (cast `/Game/Dynamic/ThirdPerson/Blueprints/BP_ThirdPersonCharacter` (`self.GetAvatarActorFromActorInfo`)))
  (set `self.As TPC` _asbp_third_person_character)
  (if (`/Game/Dynamic/ThirdPerson/Blueprints/BP_ThirdPersonCharacter.Burried` _as_tpc_3)
    (set `/Game/Dynamic/ThirdPerson/Blueprints/BP_ThirdPersonCharacter.Burried` false _as_tpc_3)
    (set `CharacterMovementComponent.MaxWalkSpeed` (`/Game/Dynamic/Creatures/CreatureDataAsset.Speed` _thiscreature) (`Character.CharacterMovement` _as_tpc_3))
    (set `Character.JumpMaxCount` (`/Game/Dynamic/Creatures/CreatureDataAsset.NumOfJumps` _thiscreature) _as_tpc)
    (`SkeletalMeshComponent.SetSkeletalMeshAsset` (`Character.Mesh` _as_tpc) (`/Game/Dynamic/Creatures/CreatureDataAsset.Model` _thiscreature))
    (`MovementComponent.StopMovementImmediately` _charactermovement)
    (set `CharacterMovementComponent.MaxWalkSpeed` 25.0 _charactermovement)
    (`KismetSystemLibrary.Delay` 1.4)
    (set `CharacterMovementComponent.MaxWalkSpeed` (`/Game/Dynamic/Creatures/CreatureDataAsset.Speed` (`/Game/Dynamic/ThirdPerson/Blueprints/BP_ThirdPersonCharacter.ThisCreature` _as_tpc_2)) _charactermovement)
    (`self.K2_EndAbility`)
    (else
      (`self.K2_EndAbility`))))