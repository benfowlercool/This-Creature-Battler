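; Template Gameplay Ability with shared cooldown helpers for attacks, abilities and bury.
; On activation it commits, caches the avatar as BP_ThirdPersonCharacter, then ends immediately.
; Uncalled here, the helpers decrement a counter, update the WBMain widget and remove a gameplay tag at zero, most also ending the ability.
; All but BurryTimer share A1Timer, and all but CooldownTimerAttack1 update the Attack2 display.
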(event `self.K2_ActivateAbility`
  (`self.K2_CommitAbility`)
  (bind _asbp_third_person_character (cast `/Game/Dynamic/ThirdPerson/Blueprints/BP_ThirdPersonCharacter` (`self.GetAvatarActorFromActorInfo`)))
  (set `self.As TPC` _asbp_third_person_character)
  (`self.K2_EndAbility`))

(fn `BurryTimer`
  (params (Tag :type "GameplayTag Structure") (`Max Timer` :type "Float (double-precision)"))
  (set `self.Tag` Tag)
  (set `self.MaxTimer` `Max Timer`)
  (if (> (`self.BuryCC`) 0.0)
    (bind _result (`/Engine/EditorBlueprintResources/StandardMacros.DecrementFloat` (`self.BuryCC`))
      (:`  `
        (`/Game/Dynamic/UI/WB_CharData.UpdateAttack2` (`/Game/Dynamic/ThirdPerson/Blueprints/BP_ThirdPersonCharacter.WB_Main` (`self.As TPC`)) (`self.BuryCC`) (`self.MaxTimer`))
        (if (== _result 0.0)
          (`BlueprintGameplayTagLibrary.RemoveGameplayTag` (`/Game/Dynamic/ThirdPerson/Blueprints/BP_ThirdPersonCharacter.GameplayTagManager` (`self.As TPC`)) (`self.Tag`))
          (`self.K2_EndAbility`))))))

(fn `CooldownTimerAbility1`
  (params (Tag :type "GameplayTag Structure") (`Max Timer` :type "Float (double-precision)"))
  (set `self.Tag` Tag)
  (set `self.MaxTimer` `Max Timer`)
  (if (> (`self.A1Timer`) 0.0)
    (bind _result (`/Engine/EditorBlueprintResources/StandardMacros.DecrementFloat` (`self.A1Timer`))
      (:`  `
        (`/Game/Dynamic/UI/WB_CharData.UpdateAttack2` (`/Game/Dynamic/ThirdPerson/Blueprints/BP_ThirdPersonCharacter.WB_Main` (`self.As TPC`)) (`self.A1Timer`) (`self.MaxTimer`))
        (if (== _result 0.0)
          (`BlueprintGameplayTagLibrary.RemoveGameplayTag` (`/Game/Dynamic/ThirdPerson/Blueprints/BP_ThirdPersonCharacter.GameplayTagManager` (`self.As TPC`)) (`self.Tag`))
          (return))))))

(fn `CooldownTimerAttack1`
  (params (Tag :type "GameplayTag Structure") (`Max Timer` :type "Float (double-precision)"))
  (set `self.Tag` Tag)
  (set `self.MaxTimer` `Max Timer`)
  (if (> (`self.A1Timer`) 0.0)
    (bind _result (`/Engine/EditorBlueprintResources/StandardMacros.DecrementFloat` (`self.A1Timer`))
      (:`  `
        (`/Game/Dynamic/UI/WB_CharData.UpdateAttack1` (`/Game/Dynamic/ThirdPerson/Blueprints/BP_ThirdPersonCharacter.WB_Main` (`self.As TPC`)) (`self.A1Timer`) (`self.MaxTimer`))
        (if (== _result 0.0)
          (`BlueprintGameplayTagLibrary.RemoveGameplayTag` (`/Game/Dynamic/ThirdPerson/Blueprints/BP_ThirdPersonCharacter.GameplayTagManager` (`self.As TPC`)) (`self.Tag`))
          (`self.K2_EndAbility`))))))

(fn `CooldownTimerAttack2`
  (params (Tag :type "GameplayTag Structure") (`Max Timer` :type "Float (double-precision)"))
  (set `self.Tag` Tag)
  (set `self.MaxTimer` `Max Timer`)
  (if (> (`self.A1Timer`) 0.0)
    (bind _result (`/Engine/EditorBlueprintResources/StandardMacros.DecrementFloat` (`self.A1Timer`))
      (:`  `
        (`/Game/Dynamic/UI/WB_CharData.UpdateAttack2` (`/Game/Dynamic/ThirdPerson/Blueprints/BP_ThirdPersonCharacter.WB_Main` (`self.As TPC`)) (`self.A1Timer`) (`self.MaxTimer`))
        (if (== _result 0.0)
          (`BlueprintGameplayTagLibrary.RemoveGameplayTag` (`/Game/Dynamic/ThirdPerson/Blueprints/BP_ThirdPersonCharacter.GameplayTagManager` (`self.As TPC`)) (`self.Tag`))
          (`self.K2_EndAbility`))))))