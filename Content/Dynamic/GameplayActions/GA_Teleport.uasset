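; GA_Teleport is a gameplay ability that teleports the player's BP_ThirdPersonCharacter to an aimed location.
; On activation it casts the avatar actor to that character, commits the ability and calls UnAim on it.
; If the character has HitDetected set, it moves the actor to HitDetectLocation without sweeping, then ends the ability either way.
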(event `self.K2_ActivateAbility`
  (bind _as_tpc (`self.As TPC`))
  (bind _asbp_third_person_character (cast `/Game/Dynamic/ThirdPerson/Blueprints/BP_ThirdPersonCharacter` (`self.GetAvatarActorFromActorInfo`)))
  (set `self.As TPC` _asbp_third_person_character)
  (`self.K2_CommitAbility`)
  (`/Game/Dynamic/ThirdPerson/Blueprints/BP_ThirdPersonCharacter.UnAim` _as_tpc)
  (if (`/Game/Dynamic/ThirdPerson/Blueprints/BP_ThirdPersonCharacter.HitDetected` _as_tpc)
    (`Actor.K2_SetActorLocation` _as_tpc (`/Game/Dynamic/ThirdPerson/Blueprints/BP_ThirdPersonCharacter.hitDetectLocation` _as_tpc) false true)
    (`self.K2_EndAbility`)
    (else
      (`self.K2_EndAbility`))))