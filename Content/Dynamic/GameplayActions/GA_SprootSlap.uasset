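; Gameplay ability for the Sproot slap, the third-person character's first attack.
; On activation it adds the Attacking.Attack1 tag to the character's tag container and plays the attack montage.
; It then starts a fast looping timer that calls CooldownTimerAttack1 with the character's regular Attack1 cooldown maximum.
; A Burried tag check exists, but both branches behave identically and the buried cooldown setup is never reached.
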(event `UpdateTimerBurried`
  (`self.CooldownTimerAttack1` (struct :`TagName` "Attacking?.Attack1") (`/Game/Dynamic/ThirdPerson/Blueprints/BP_ThirdPersonCharacter.Attack1MC_Burried` (`self.As TPC`))))

(event `self.K2_ActivateAbility`
  (bind _as_tpc (`self.As TPC`))
  (bind _asbp_third_person_character (cast `/Game/Dynamic/ThirdPerson/Blueprints/BP_ThirdPersonCharacter` (`self.GetAvatarActorFromActorInfo`)))
  (bind _output_get (set `self.As TPC` _asbp_third_person_character))
  (`BlueprintGameplayTagLibrary.AddGameplayTag` (`/Game/Dynamic/ThirdPerson/Blueprints/BP_ThirdPersonCharacter.GameplayTagManager` _output_get) (struct :`TagName` "Attacking?.Attack1"))
  (if (`BlueprintGameplayTagLibrary.HasTag` (`/Game/Dynamic/ThirdPerson/Blueprints/BP_ThirdPersonCharacter.GameplayTagManager` _as_tpc) (struct :`TagName` "Burried"))
    _
    (else
      _))
  (`|PlayMontage` (`Character.Mesh` (`self.As TPC`)) "/Game/Static/Characters/Models/Sproot/AttackMontage1.AttackMontage1"
    (:`then`
      (set `self.A1Timer` (`/Game/Dynamic/ThirdPerson/Blueprints/BP_ThirdPersonCharacter.Attack1MC` _as_tpc))
      (`KismetSystemLibrary.K2_SetTimerDelegate` (delegate `UpdateTimerReg`) 0.001 true))))

(event `UpdateTimerReg`
  (`self.CooldownTimerAttack1` (struct :`TagName` "Attacking?.Attack1") (`/Game/Dynamic/ThirdPerson/Blueprints/BP_ThirdPersonCharacter.Attack1MC` (`self.As TPC`))))