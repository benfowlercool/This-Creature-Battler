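; GA_Fireball is a creature gameplay ability that, despite its name, spawns no fireball in this graph and only updates the avatar's walk speed.
; On activation it casts the avatar to BP_ThirdPersonCharacter and commits.
; Unless the character is tagged Burried, it sets MaxWalkSpeed from the creature's Speed stat, boosted when tagged Sprinting, then ends.
; When Burried, the ability is never explicitly ended.
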(event `self.K2_ActivateAbility`
  (bind _as_tpc (`self.As TPC`))
  (bind _charactermovement (`Character.CharacterMovement` _as_tpc))
  (bind _gameplaytagmanager (`/Game/Dynamic/ThirdPerson/Blueprints/BP_ThirdPersonCharacter.GameplayTagManager` _as_tpc))
  (bind _speed (`/Game/Dynamic/Creatures/CreatureDataAsset.Speed` (`/Game/Dynamic/ThirdPerson/Blueprints/BP_ThirdPersonCharacter.ThisCreature` _as_tpc)))
  (bind _asbp_third_person_character (cast `/Game/Dynamic/ThirdPerson/Blueprints/BP_ThirdPersonCharacter` (`self.GetAvatarActorFromActorInfo`)))
  (set `self.As TPC` _asbp_third_person_character)
  (`self.K2_CommitAbility`)
  (if (not (`BlueprintGameplayTagLibrary.HasTag` _gameplaytagmanager (struct :`TagName` "Burried")))
    (if (`BlueprintGameplayTagLibrary.HasTag` _gameplaytagmanager (struct :`TagName` "Sprinting"))
      (set `CharacterMovementComponent.MaxWalkSpeed` (* _speed 1.9) _charactermovement)
      (else
        (set `CharacterMovementComponent.MaxWalkSpeed` _speed _charactermovement)))
    (`self.K2_EndAbility`)))