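; GA_SprootSlap is a Gameplay Ability that triggers the Sproot creature's slap as an Attack1 action.
; On activation it casts the avatar to BP_ThirdPersonCharacter and adds the Attacking.Attack1 tag to its GameplayTagManager container, unless already present.
; It then plays the attack montage on the mesh unless the character is tagged Burried.
; The graph itself neither removes the tag nor ends the ability.
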(event `self.K2_ActivateAbility`
  (bind _as_tpc (`self.As TPC`))
  (bind _asbp_third_person_character (cast `/Game/Dynamic/ThirdPerson/Blueprints/BP_ThirdPersonCharacter` (`self.GetAvatarActorFromActorInfo`)))
  (bind _output_get (set `self.As TPC` _asbp_third_person_character))
  (if (not (`BlueprintGameplayTagLibrary.HasTag` (`/Game/Dynamic/ThirdPerson/Blueprints/BP_ThirdPersonCharacter.GameplayTagManager` _output_get) (struct :`TagName` "Attacking?.Attack1")))
    (`BlueprintGameplayTagLibrary.AddGameplayTag` (`/Game/Dynamic/ThirdPerson/Blueprints/BP_ThirdPersonCharacter.GameplayTagManager` _as_tpc) (struct :`TagName` "Attacking?.Attack1"))
    (if (not (`BlueprintGameplayTagLibrary.HasTag` (`/Game/Dynamic/ThirdPerson/Blueprints/BP_ThirdPersonCharacter.GameplayTagManager` _as_tpc) (struct :`TagName` "Burried")))
      (`|PlayMontage` (`Character.Mesh` (`self.As TPC`)) "/Game/Static/Characters/Models/Sproot/SprootAttackMontage.SprootAttackMontage"))))