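; GA_WarlockProj is a Gameplay Ability for the Attack1 creature action that fires a rapid burst of BP_AdamWarlockProj projectiles.
; On activation it adds the Attacking.Attack1 tag to the character's tag container and commits the ability.
; A short-delay loop spawns projectiles at the character's location along the follow camera's rotation until a counter passes its limit, then ends the ability.
; The counter is never reset in this graph.
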(event `self.K2_ActivateAbility`
  (bind _numofprojectiles (`self.numOfProjectiles`))
  (bind _asbp_third_person_character (cast `/Game/Dynamic/ThirdPerson/Blueprints/BP_ThirdPersonCharacter` (`self.GetAvatarActorFromActorInfo`)))
  (bind _output_get (set `self.As TPC` _asbp_third_person_character))
  (`BlueprintGameplayTagLibrary.AddGameplayTag` (`/Game/Dynamic/ThirdPerson/Blueprints/BP_ThirdPersonCharacter.GameplayTagManager` _output_get) (struct :`TagName` "Attacking?.Attack1"))
  (`self.K2_CommitAbility`)
  (bind (_returnvalue_location _returnvalue_rotation _returnvalue_scale) (`KismetMathLibrary.BreakTransform` (`Actor.GetTransform` _output_get)))
  (`|SpawnActorFromClass` "/Game/Dynamic/Projectiles/BP_AdamWarlockProj.BP_AdamWarlockProj_C" (`KismetMathLibrary.MakeTransform` _returnvalue_location (`SceneComponent.K2_GetComponentRotation` (`/Game/Dynamic/ThirdPerson/Blueprints/BP_ThirdPersonCharacter.FollowCamera` _output_get)) _returnvalue_scale) "Undefined" "MultiplyWithRoot" _output_get _output_get :!label _label)
  (`KismetSystemLibrary.Delay` 0.07)
  (if (<= _numofprojectiles 3)
    (`/Engine/EditorBlueprintResources/StandardMacros.IncrementInt` _numofprojectiles
      (:`  `
        (goto _label)))
    (else
      (`self.K2_EndAbility`))))