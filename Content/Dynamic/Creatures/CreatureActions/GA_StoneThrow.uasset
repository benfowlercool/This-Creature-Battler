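; Gameplay ability for a creature stone throw that toggles between aiming and throwing through gameplay tags on the third-person character.
; It commits and adds the Attacking.Ability1 tag, then adds ADS if absent, leaving the ability unended.
; If ADS is already present, it spawns a BP_Pebble at the character's transform, removes ADS and ends.
; Attacking.Ability1 is not removed here, and the UnAim call is disconnected.
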(event `self.K2_ActivateAbility`
  (bind _gameplaytagmanager (`/Game/Dynamic/ThirdPerson/Blueprints/BP_ThirdPersonCharacter.GameplayTagManager` (`self.As TPC`)))
  (bind _asbp_third_person_character (cast `/Game/Dynamic/ThirdPerson/Blueprints/BP_ThirdPersonCharacter` (`self.GetAvatarActorFromActorInfo`)))
  (bind _output_get (set `self.As TPC` _asbp_third_person_character))
  (`self.K2_CommitAbility`)
  (bind _gameplaytagmanager_2 (`/Game/Dynamic/ThirdPerson/Blueprints/BP_ThirdPersonCharacter.GameplayTagManager` _output_get))
  (`BlueprintGameplayTagLibrary.AddGameplayTag` _gameplaytagmanager_2 (struct :`TagName` "Attacking?.Ability1"))
  (if (`BlueprintGameplayTagLibrary.HasTag` _gameplaytagmanager_2 (struct :`TagName` "ADS"))
    (`|SpawnActorFromClass` "/Game/Dynamic/ThirdPerson/Blueprints/BP_Pebble.BP_Pebble_C" (`Actor.GetTransform` (`self.As TPC`)) "Undefined" "MultiplyWithRoot" null null)
    (`BlueprintGameplayTagLibrary.RemoveGameplayTag` _gameplaytagmanager (struct :`TagName` "ADS"))
    (`self.K2_EndAbility`)
    (else
      (`BlueprintGameplayTagLibrary.AddGameplayTag` _gameplaytagmanager (struct :`TagName` "ADS")))))