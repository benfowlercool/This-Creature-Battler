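; Gameplay ability for the poison plant attack, used as a character's Attack2 slot.
; On activation it commits, adds the Attack2 tag and spawns a double-scale BP_Plant at the character's XY and rotation.
; The spawn Z is FindFloor's line distance itself, not an offset from the character.
; It then seeds the cooldown from Attack2MC and runs a very fast looping timer that calls CooldownTimerAttack2.
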(event `self.K2_ActivateAbility`
  (bind _asbp_third_person_character (cast `/Game/Dynamic/ThirdPerson/Blueprints/BP_ThirdPersonCharacter` (`self.GetAvatarActorFromActorInfo`)))
  (bind _output_get (set `self.As TPC` _asbp_third_person_character))
  (`self.K2_CommitAbility`)
  (`BlueprintGameplayTagLibrary.AddGameplayTag` (`/Game/Dynamic/ThirdPerson/Blueprints/BP_ThirdPersonCharacter.GameplayTagManager` _output_get) (struct :`TagName` "Attacking?.Attack2"))
  (bind (_returnvalue_x _returnvalue_y) (`KismetMathLibrary.BreakVector` (`Actor.K2_GetActorLocation` _output_get)))
  (bind (_floorresult_bblockinghit _floorresult_bwalkablefloor _floorresult_blinetrace _floorresult_floordist _floorresult_linedist) (break `FindFloorResult` (`CharacterMovementComponent.K2_FindFloor` (`Character.CharacterMovement` _output_get) (`Actor.K2_GetActorLocation` _output_get))))
  (`|SpawnActorFromClass` "/Game/Dynamic/ThirdPerson/Blueprints/BP_Plant.BP_Plant_C" (`KismetMathLibrary.MakeTransform` (`KismetMathLibrary.MakeVector` _returnvalue_x _returnvalue_y _floorresult_linedist) (`Actor.K2_GetActorRotation` _output_get) (2.0 2.0 2.0)) "Undefined" "MultiplyWithRoot" null null)
  (set `self.A1Timer` (`/Game/Dynamic/ThirdPerson/Blueprints/BP_ThirdPersonCharacter.Attack2MC` (`self.As TPC`)))
  (`KismetSystemLibrary.K2_SetTimerDelegate` (delegate `UpdateTimerReg`) 0.001 true))

(event `UpdateTimerReg`
  (`self.CooldownTimerAttack2` (struct :`TagName` "Attacking?.Attack2") (`/Game/Dynamic/ThirdPerson/Blueprints/BP_ThirdPersonCharacter.Attack2MC` (`self.As TPC`))))