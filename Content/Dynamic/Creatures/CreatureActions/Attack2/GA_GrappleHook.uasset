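; Gameplay ability that toggles a grappling hook on the character, using a Grappling gameplay tag as the state.
; Activation line-traces from the follow camera; a hit stores the grapple point, adds the tag, sets Flying movement and shows the cable.
; Reactivation while tagged removes the tag, hides the cable and restores Walking.
; The ability ends immediately after either change, but a missed trace never calls EndAbility.
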(event `self.K2_ActivateAbility`
  (bind _as_tpc (`self.As TPC`))
  (bind _as_tpc_2 (`self.As TPC`))
  (bind _followcamera (`/Game/Dynamic/ThirdPerson/Blueprints/BP_ThirdPersonCharacter.FollowCamera` _as_tpc_2))
  (bind _returnvalue (`SceneComponent.K2_GetComponentLocation` _followcamera))
  (`parent.K2_ActivateAbility`)
  (if (`BlueprintGameplayTagLibrary.HasTag` (`/Game/Dynamic/ThirdPerson/Blueprints/BP_ThirdPersonCharacter.GameplayTagManager` _as_tpc_2) (struct :`TagName` "Grappling"))
    (`BlueprintGameplayTagLibrary.RemoveGameplayTag` (`/Game/Dynamic/ThirdPerson/Blueprints/BP_ThirdPersonCharacter.GameplayTagManager` (`self.As TPC`)) (struct :`TagName` "Grappling"))
    (`SceneComponent.SetVisibility` (`/Game/Dynamic/ThirdPerson/Blueprints/BP_ThirdPersonCharacter.GrappleCable` (`self.As TPC`)) false false)
    (`CharacterMovementComponent.SetMovementMode` (`Character.CharacterMovement` (`self.As TPC`)) "MOVE_Walking" 0)
    (`self.K2_EndAbility`)
    (else
      (bind (_outhit _returnvalue_2) (`KismetSystemLibrary.LineTraceSingle` :`Start` _returnvalue :`End` (+ _returnvalue (* (`KismetMathLibrary.GetForwardVector` (`SceneComponent.K2_GetComponentRotation` _followcamera)) 2500.0)) :`TraceChannel` "TraceTypeQuery1" :`DrawDebugType` "ForDuration"))
      (if _returnvalue_2
        (set `/Game/Dynamic/ThirdPerson/Blueprints/BP_ThirdPersonCharacter.GrapplePoint` (`.ImpactPoint` (`GameplayStatics.BreakHitResult` _outhit)) (`self.As TPC`))
        (`BlueprintGameplayTagLibrary.AddGameplayTag` (`/Game/Dynamic/ThirdPerson/Blueprints/BP_ThirdPersonCharacter.GameplayTagManager` _as_tpc) (struct :`TagName` "Grappling"))
        (`CharacterMovementComponent.SetMovementMode` (`Character.CharacterMovement` _as_tpc) "MOVE_Flying" 0)
        (`SceneComponent.SetVisibility` (`/Game/Dynamic/ThirdPerson/Blueprints/BP_ThirdPersonCharacter.GrappleCable` (`self.As TPC`)) true false)
        (`self.K2_EndAbility`)))))