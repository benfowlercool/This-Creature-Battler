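; BP_SlowWeb is a web actor, apparently meant to slow enemies, though no slowing logic is present.
; On BeginPlay it starts a timed self-destruct and runs one debug-drawn sphere trace for pawns, casting the hit to BP_EnemyAITemplate without further action.
; Tick clears an enemy reference every frame.
; A destroy-on-damage handler exists, but its binding is never executed.
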(event `self.ReceiveBeginPlay`
  (bind _returnvalue (`self.K2_GetActorLocation`))
  (`|ExecutionSequence`
    (:`then_0`
      (`KismetSystemLibrary.Delay` 100.0)
      (`self.K2_DestroyActor`))
    (:`then_1`
      (bind (_outhit _returnvalue_2) (`KismetSystemLibrary.SphereTraceSingleForObjects` :`Start` _returnvalue :`End` _returnvalue :`Radius` 490.0 :`ObjectTypes` (`|MakeArray` "ObjectTypeQuery3" :!type "EObjectTypeQuery Enum") :`DrawDebugType` "ForDuration" :`DrawTime` 8.0))
      (if _returnvalue_2
        (cast `/Game/Dynamic/AI/BP_EnemyAITemplate` (`.HitActor` (`GameplayStatics.BreakHitResult` _outhit)))))))

(event `self.ReceiveTick`
  (params (DeltaSeconds :type "Float (single-precision)"))
  (set `self.As BP Enemy AITemplate` null))

(event `OnTakeAnyDamage_Event` :!signature `self.OnTakeAnyDamage`
  (params (DamagedActor :type "Actor Object Reference") (Damage :type "Float (single-precision)") (DamageType :type "DamageType Object Reference") (InstigatedBy :type "Controller Object Reference") (DamageCauser :type "Actor Object Reference"))
  (`self.K2_DestroyActor`))

(fn `UserConstructionScript`)