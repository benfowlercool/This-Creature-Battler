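; BP_HomingProjectile is a projectile that homes in on enemies, damages Enemy-tagged actors on hit, and explodes on contact with anything except the player.
; Every 0.1 seconds it scans all BP_EnemyAITemplate actors and points ProjectileMovement homing at the chosen one's Origin component.
; Target selection keeps the smallest distance in the Dist variable, which is never reset between scans.
; If still alive after one second, it explodes and destroys itself.
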(event `self.ReceiveHit`
  (params (MyComp :type "PrimitiveComponent Object Reference") (Other :type "Actor Object Reference") (OtherComp :type "PrimitiveComponent Object Reference") (bSelfMoved :type Boolean) (HitLocation :type "Vector Structure") (HitNormal :type "Vector Structure") (NormalImpulse :type "Vector Structure") (Hit :type "HitResult Structure (by ref)"))
  (if (not (== (`GameplayStatics.GetPlayerCharacter` 0) Other))
    (if (`self.ActorHasTag` Other "Enemy")
      (`GameplayStatics.ApplyDamage` Other (`self.Damage`)))
    (`GameplayStatics.SpawnEmitterAtLocation` "/Game/Static/StarterContent/Particles/P_Explosion.P_Explosion" (`self.K2_GetActorLocation`) (struct) (0.5 0.5 0.5) :!label _label)
    (`self.K2_DestroyActor`)))

(event `self.ReceiveBeginPlay`
  (`|ExecutionSequence`
    (:`then_0`
      (`KismetSystemLibrary.Delay` 1.0)
      (`/Engine/EditorBlueprintResources/StandardMacros.IsValid` self
        (:`Is Valid`
          (goto _label))))
    (:`then_1`
      (`self.LockOn` :!label _label_2)
      (`KismetSystemLibrary.Delay` 0.1)
      (goto _label_2))))

(event `LockOn`
  (bind _projectilemovement (`self.ProjectileMovement`))
  (bind _homingtarget (`self.Homing`))
  (set `ProjectileMovementComponent.HomingTargetComponent` _homingtarget _projectilemovement)
  (set `ProjectileMovementComponent.bIsHomingProjectile` true _projectilemovement)
  (set `ProjectileMovementComponent.HomingAccelerationMagnitude` 10000.0 _projectilemovement))

(fn `Homing`
  (returns (HomingTarget :type "SceneComponent Object Reference"))
  (bind _outactors (`GameplayStatics.GetAllActorsOfClass` "/Game/Dynamic/AI/BP_EnemyAITemplate.BP_EnemyAITemplate_C"))
  (for _array_element _outactors
    (bind _returnvalue (`KismetMathLibrary.VSize` (- (`self.K2_GetActorLocation` _array_element) (`self.K2_GetActorLocation`))))
    (if (< _returnvalue (`self.Dist`))
      (set `self.Dist` _returnvalue)
      (set `self.Target` _array_element)))
  (bind _target (`self.Target`)
    (:`then`
      (bind _origin (`/Game/Dynamic/AI/BP_EnemyAITemplate.Origin` _target))
      (if (`KismetSystemLibrary.IsValid` _origin)
        (return _origin)))
    (:`else`)))

(fn `UserConstructionScript`)