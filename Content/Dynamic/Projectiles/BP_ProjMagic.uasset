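; Magic projectile that damages enemies and explodes on impact or after a short fuse, ignoring hits on player character 0.
; Actors tagged Enemy take direct damage.
; Other hits and the BeginPlay delay share a splash path: a debug-drawn single-result pawn sphere trace applies reduced damage to an enemy AI and launches it using a scaled look-at rotation as velocity.
; Both paths spawn an explosion emitter and destroy the projectile.
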(event `self.ReceiveHit`
  (params (MyComp :type "PrimitiveComponent Object Reference") (Other :type "Actor Object Reference") (OtherComp :type "PrimitiveComponent Object Reference") (bSelfMoved :type Boolean) (HitLocation :type "Vector Structure") (HitNormal :type "Vector Structure") (NormalImpulse :type "Vector Structure") (Hit :type "HitResult Structure (by ref)"))
  (bind _returnvalue (`self.K2_GetActorLocation`))
  (if (== (`GameplayStatics.GetPlayerCharacter` 0) Other)
    _
    (elif (`self.ActorHasTag` Other "Enemy")
      (`GameplayStatics.ApplyDamage` Other (`self.DamageTotal`))
      (`GameplayStatics.SpawnEmitterAtLocation` "/Game/Static/StarterContent/Particles/P_Explosion.P_Explosion" _returnvalue (struct) (2.0 2.0 2.0) :!label _label)
      (`self.K2_DestroyActor`)
      (else
        (bind (_outhit _returnvalue_2) (`KismetSystemLibrary.SphereTraceSingleForObjects` :`Start` _returnvalue :`End` _returnvalue :`Radius` 200.0 :`ObjectTypes` (`|MakeArray` "ObjectTypeQuery3" :!type "EObjectTypeQuery Enum") :`DrawDebugType` "ForDuration" :!label _label_2))
        (`|ExecutionSequence`
          (:`then_0`
            (if _returnvalue_2
              (bind _asbp_enemy_aitemplate (cast `/Game/Dynamic/AI/BP_EnemyAITemplate` (`.HitActor` (`GameplayStatics.BreakHitResult` _outhit))))
              (`Character.LaunchCharacter` _asbp_enemy_aitemplate (* (`KismetMathLibrary.FindLookAtRotation` _returnvalue (`self.K2_GetActorLocation` _asbp_enemy_aitemplate)) (100.0 100.0 100.0)) false false)
              (`GameplayStatics.ApplyDamage` _asbp_enemy_aitemplate (/ (`self.DamageTotal`) (`self.DamageSplashFalloff`)) null null "/Script/Engine.DamageType")
              (`self.K2_DestroyActor`)))
          (:`then_1`
            (goto _label)))))))

(event `self.ReceiveBeginPlay`
  (`KismetSystemLibrary.Delay` 0.7)
  (`/Engine/EditorBlueprintResources/StandardMacros.IsValid` self
    (:`Is Valid`
      (goto _label_2))))

(fn `UserConstructionScript`)