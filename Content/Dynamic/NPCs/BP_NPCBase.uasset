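; Base NPC Blueprint that shows a line-by-line dialogue when Talkto is called.
; Each call creates a WB_Dialogue widget if needed, displays the next Dialogue entry, and removes the widget after the last line.
; Tick polls TriggerZone for an overlapping BP_PlayerOverworld, using a resettable DoOnce to close the dialogue and reset its index once the player leaves.
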(event `/Game/Dynamic/NPCs/Dialogue/BP_Dialogue.TalkTo`
  (`self.UI`
    (:`then`
      (if (not (`Widget.IsInViewport` (`self.UI`)))
        (set `self.TalkIndex` 0)
        (set `self.UI` null)))
    (:`else`
      _))
  (if (< (`self.TalkIndex`) (`KismetArrayLibrary.Array_Length` (`self.dialogue`)))
    (`self.UI`
      (:`then`
        _)
      (:`else`
        (bind _returnvalue (`|CreateWidget` "/Game/Dynamic/UI/WB_Dialogue.WB_Dialogue_C" (`GameplayStatics.GetPlayerController` 0)))
        (bind _output_get (set `self.UI` _returnvalue))
        (`UserWidget.AddToViewport` _output_get 0)))
    (`TextBlock.SetText` (`/Game/Dynamic/UI/WB_Dialogue.DialogueText` (`self.UI`)) (`KismetTextLibrary.Conv_StringToText` (`|GetArrayItem` (`self.dialogue`) (`self.TalkIndex`))))
    (`/Engine/EditorBlueprintResources/StandardMacros.IncrementInt` (`self.TalkIndex`))
    (else
      (`Widget.RemoveFromParent` (`self.UI`))
      (set `self.TalkIndex` 0)
      (set `self.UI` null))))

(event `self.ReceiveTick`
  (params (DeltaSeconds :type "Float (single-precision)"))
  (if (`KismetSystemLibrary.IsValid` (`|GetArrayItem` (`PrimitiveComponent.GetOverlappingActors` (`self.TriggerZone`) "/Game/Dynamic/ThirdPerson/Blueprints/BP_PlayerOverworld.BP_PlayerOverworld_C")))
    (goto _label :!via `Reset`)
    (else
      (`/Engine/EditorBlueprintResources/StandardMacros.DoOnce` false :!label _label
        (:`Completed`
          (bind _ui (`self.UI`)
            (:`then`
              (`Widget.RemoveFromParent` _ui)
              (set `self.TalkIndex` 0)
              (set `self.UI` null))
            (:`else`)))))))

(fn `UserConstructionScript`)