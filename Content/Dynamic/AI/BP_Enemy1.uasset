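; BP_Enemy1 is an enemy Blueprint that tracks health, shows it on a health bar widget and plays a death montage.
; On BeginPlay it caches the WB_Enemy widget and initializes current health.
; AnyDamage subtracts health and updates the bar, playing the montage at zero or below and setting Dead when it completes.
; Each hit also binds a death event to a handler that does nothing yet.
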(event `self.ReceiveBeginPlay`
  (bind _health (`self.Health`))
  (bind _aswb_enemy (cast `/Game/Dynamic/UI/WB_Enemy` (`WidgetComponent.GetUserWidgetObject` (`self.Healthbar`))))
  (set `self.WB_Enemy` _aswb_enemy)
  (bind _output_get (set `self.CurrHealth` _health))
  (`/Game/Dynamic/UI/WB_Enemy.UpdateHealthUI` (`self.WB_Enemy`) _output_get _health))

(event `self.ReceiveAnyDamage`
  (params (Damage :type "Float (single-precision)") (DamageType :type "DamageType Object Reference") (InstigatedBy :type "Controller Object Reference") (DamageCauser :type "Actor Object Reference"))
  (bind _output_get (set `self.CurrHealth` (- (`self.CurrHealth`) Damage)))
  (`|ExecutionSequence`
    (:`then_0`
      (if (<= _output_get 0.0)
        (`KismetSystemLibrary.PrintText` "dead")
        (`|PlayMontage` (`self.Mesh`) "/Game/Static/Characters/Mannequins/Animations/Manny/death_montage.death_montage"
          (:`OnCompleted`
            (set `self.Dead` true)))
        (else
          (`KismetSystemLibrary.PrintString` (`KismetStringLibrary.Conv_DoubleToString` _output_get)))))
    (:`then_1`
      (`/Game/Dynamic/UI/WB_Enemy.UpdateHealthUI` (`self.WB_Enemy`) _output_get (`self.Health`))
      (add `self.DeathEvent` (delegate `CustomEvent`)))))

(event `CustomEvent` :!signature `self.DeathEvent`
  (params (Death :type Boolean))
  (if Death
    _))

(fn `UserConstructionScript`)