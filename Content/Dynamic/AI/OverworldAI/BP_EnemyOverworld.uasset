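; Overworld enemy that appears as a random creature and triggers a level change when the player touches it.
; On BeginPlay it hides its healthbar, picks a creature from CreatureList, and applies that creature's mesh, anim class and randomly varied scale.
; Player overlap with its sphere resets the creature's EnemyIndex, saves and prints the player's transform via the Game_Vars game instance, then opens ThirdPersonMap.
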(event `self.ReceiveBeginPlay`
  (`parent.ReceiveBeginPlay`)
  (`SceneComponent.SetVisibility` (`self.Healthbar`) false false)
  (for _array_element (`/Game/Dynamic/Creatures/CreatureCollection.CreatureArray` (`self.CreatureList`))
    (`KismetArrayLibrary.Array_Add` (`self.Creatures`) _array_element))
  (bind _output_get (set `self.This Creature` (`KismetArrayLibrary.Array_Random` (`self.Creatures`))))
  (`SkeletalMeshComponent.SetSkeletalMeshAsset` (`self.Mesh`) (`/Game/Dynamic/Creatures/CreatureDataAsset.Model` _output_get))
  (`SkeletalMeshComponent.SetAnimInstanceClass` (`self.Mesh`) (`/Game/Dynamic/Creatures/CreatureDataAsset.CreatureAnimationBlueprint` _output_get))
  (`SceneComponent.SetWorldScale3D` (`self.Mesh`) (* (`/Game/Dynamic/Creatures/CreatureDataAsset.Scale` (`self.This Creature`)) (+ (/ (`KismetMathLibrary.Conv_IntToDouble` (`KismetMathLibrary.RandomIntegerInRange` -12 12)) 96) 1.0))))

(event `self.Sphere_0.OnComponentBeginOverlap`
  (params (OverlappedComponent :type "PrimitiveComponent Object Reference") (OtherActor :type "Actor Object Reference") (OtherComp :type "PrimitiveComponent Object Reference") (OtherBodyIndex :type Integer) (bFromSweep :type Boolean) (SweepResult :type "HitResult Structure (by ref)"))
  (cast `/Game/Dynamic/ThirdPerson/Blueprints/BP_ThirdPersonCharacter` OtherActor)
  (set `/Game/Dynamic/Creatures/CreatureDataAsset.EnemyIndex` 0 (`self.This Creature`))
  (bind _asgame_vars (cast `/Game/Game_Vars` (`GameplayStatics.GetGameInstance`)))
  (bind _output_get (set `/Game/Game_Vars.playerPosition` (`self.GetTransform` OtherActor) _asgame_vars))
  (`KismetSystemLibrary.PrintString` (`KismetStringLibrary.Conv_TransformToString` _output_get))
  (`GameplayStatics.OpenLevelBySoftObjectPtr` "/Game/Static/Maps/ThirdPersonMap.ThirdPersonMap"))

(fn `UserConstructionScript`
  (`parent.UserConstructionScript`))