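; BP_ItemAllocationFunctions provides AddItemToInventory, which updates a matching item in the player character's inventory.
; It loops over the inventory component's Items for an entry equal to the EnemySlot argument and prints a debug string on a match.
; A zero-quantity match is written back to its array index unchanged, while any other match has its quantity incremented.
; Each match then reloads the inventory widget from the component.
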(fn `addItemToInventory`
  (params (enemySlot :type "/Game/Dynamic/Items/BP_ItemDataAsset Object Reference") (inventoryWidget :type "/Game/Dynamic/UI/WB_Inventory Object Reference") (NewParam :type "/Game/Dynamic/ThirdPerson/Blueprints/BP_PlayerOverworld Object Reference"))
  (locals (`Player Character` :type "/Game/Dynamic/ThirdPerson/Blueprints/BP_PlayerOverworld Object Reference"))
  (bind _bp_inventorycomponent (`/Game/Dynamic/ThirdPerson/Blueprints/BP_PlayerOverworld.BP_InventoryComponent` (`local.Player Character`)))
  (bind _items (`/Game/Dynamic/ThirdPerson/Blueprints/BP_InventoryComponent.Items` _bp_inventorycomponent))
  (set `local.Player Character` NewParam)
  (for (_array_element _array_index) _items
    (if (== _array_element enemySlot)
      (`KismetSystemLibrary.PrintString` _array_element)
      (bind _quantity (`/Game/Dynamic/Items/BP_ItemDataAsset.Quantity` _array_element))
      (if (== _quantity 0)
        (`KismetArrayLibrary.Array_Set` _items _array_index _array_element)
        (else
          (set `/Game/Dynamic/Items/BP_ItemDataAsset.Quantity` (+ _quantity 1) _array_element)))
      (`/Game/Dynamic/UI/WB_Inventory.LoadInventory` inventoryWidget _bp_inventorycomponent))))